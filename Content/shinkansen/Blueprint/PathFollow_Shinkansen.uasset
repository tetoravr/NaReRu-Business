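; Shinkansen train actor that rides PFPathFollower paths, with selectable passenger seat views and adjustable crowding.
; Timelines drive path speed for departure, speed changes and station braking, with running sound volume following along at departure and arrival.
; A "Station" overlap stops it and notifies BulletTrainWindow unless looping; Highway_End or End key switches to the "End"-tagged path.
; Seat events move Scene1 and hide that seat's passenger; BulletTrainWindow events randomly hide passengers for crowding levels.
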(event OnComponentBeginOverlap(StaticMesh)
  (params (OverlappedComponent :type Primitive%20Component%20Object%20Reference) (OtherActor :type Actor%20Object%20Reference) (OtherComp :type Primitive%20Component%20Object%20Reference) (OtherBodyIndex :type Integer) (bFromSweep :type Boolean) (SweepResult :type Hit%20Result%20Structure%20%28by%20ref%29))
  (if (Components|ComponentHasTag OtherComp "Station")
    (if (not (Variables|Default|GetStationLoop))
      (bind (_direction _speed _volume) (Timeline|タイムライン_0 PlayFromStart)
        (:Update
          (Variables|/Script/PathFollow.PFPathFollowerComponent|SetSpeedDuration (Variables|Default|GetPFPathFollower) _speed)
          (Audio|Components|Audio|SetVolumeMultiplier (Variables|Default|Get走行音) _volume :!class /Script/Engine.AudioComponent))
        (:Finished
          (bind _foundwidgets (Widget|GetAllWidgetsOfClass "/Game/shinkansen/VR_Spectator_Window/BulletTrainWindow.BulletTrainWindow_C" false))
          (Default|到着 _foundwidgets))))))

(event Custom|Highway_End
  (bind _pfpathfollower (Variables|Default|GetPFPathFollower))
  ;[1 1 1] 高速道路降りる
  (bind _outactors (Actor|GetAllActorswithTag "End"))
  (for _array_element _outactors
    (Class|PFPathFollowerComponent|SetPathOwner _pfpathfollower _array_element)
    (Variables|/Script/PathFollow.PFPathFollowerComponent|SetSpeedDuration _pfpathfollower 5e+02)
    (Class|PFPathFollowerComponent|Start _pfpathfollower 0.0)
    (Utilities|FlowControl|Delay 8e+01)
    (Class|PFPathFollowerComponent|Stop _pfpathfollower)))

(event Custom|Highway_Start
  (bind _pfpathfollower (Variables|Default|GetPFPathFollower))
  (bind _走行音 (Variables|Default|Get走行音))
  ;[1 1 1] 高速道路乗る
  (Class|PFPathFollowerComponent|Start _pfpathfollower 0.0)
  (bind (_direction _speed _発信音 _volune) (Timeline|Speed_Up PlayFromStart)
    (:Update
      (Variables|/Script/PathFollow.PFPathFollowerComponent|SetSpeedDuration _pfpathfollower _speed)
      (Audio|Components|Audio|SetVolumeMultiplier (Variables|Default|Get発進音) _発信音 :!class /Script/Engine.AudioComponent))
    (:走行音
      (Audio|Components|Audio|Play _走行音 0.0)
      (Audio|Components|Audio|SetVolumeMultiplier _走行音 _volune :!class /Script/Engine.AudioComponent))))

(event Custom|SpeedUp_75to100Km
  ;[1 1 1] 速度調節
  (bind _50_to_100 (Timeline|Speed_75%20to%20100 Play)
    (:Update
      (Variables|/Script/PathFollow.PFPathFollowerComponent|SetSpeedDuration (Variables|Default|GetPFPathFollower) _50_to_100))))

(event Custom|SpeedUP_50to75Km
  ;[1 1 1] 速度調節
  (bind _50_to_100 (Timeline|Speed_50%20to%2075 Play)
    (:Update
      (Variables|/Script/PathFollow.PFPathFollowerComponent|SetSpeedDuration (Variables|Default|GetPFPathFollower) _50_to_100))))

(event Custom|SpeedDown_100to50Km
  ;[1 1 1] 速度調節
  (bind _50_to_100 (Timeline|Speed_50%20to%20100 Reverse)
    (:Update
      (Variables|/Script/PathFollow.PFPathFollowerComponent|SetSpeedDuration (Variables|Default|GetPFPathFollower) _50_to_100))))

(event Custom|混雑度
  (|配列取得)
  (bind _foundwidgets (Widget|GetAllWidgetsOfClass "/Game/shinkansen/VR_Spectator_Window/BulletTrainWindow.BulletTrainWindow_C" false))
  (EventDispatchers|BindEventto無人 _foundwidgets (delegate Custom|無人))
  (EventDispatchers|BindEventto少数 _foundwidgets (delegate Custom|少数))
  (EventDispatchers|BindEventto普通 _foundwidgets (delegate Custom|普通))
  (EventDispatchers|BindEventto満員 _foundwidgets (delegate Custom|満員)))

(event Custom|座席E
  (Variables|Default|SetCameraPosition "-2167.000000,120.000000,247.000000")
  (Rendering|SetVisibility (Variables|Default|GetPassenger_E) false false)
  (Rendering|SetVisibility (Variables|Default|GetPassenger_D) true false)
  (Transformation|SetRelativeLocation (Variables|Default|GetScene1) (Variables|Default|GetCameraPosition) false false))

(event Custom|座席C
  (Variables|Default|SetCameraPosition "-2167.000000,-40.000000,247.000000")
  (Rendering|SetVisibility (Variables|Default|GetPassenger_C) false false)
  (Rendering|SetVisibility (Variables|Default|GetPassenger_E) true false)
  (Transformation|SetRelativeLocation (Variables|Default|GetScene1) (Variables|Default|GetCameraPosition) false false))

(event Custom|初期座席
  (Variables|Default|SetCameraPosition "-2167.000000,-80.000000,247.000000")
  (Rendering|SetVisibility (Variables|Default|GetPassenger_B) false false)
  (Rendering|SetVisibility (Variables|Default|GetPassenger_A) true false)
  (Transformation|SetRelativeLocation (Variables|Default|GetScene1) (Variables|Default|GetCameraPosition) false false))

(event Custom|座席A
  (Variables|Default|SetCameraPosition "-2167.000000,-120.000000,247.000000")
  (Rendering|SetVisibility (Variables|Default|GetPassenger_A) false false)
  (Rendering|SetVisibility (Variables|Default|GetPassenger_B) true false)
  (Transformation|SetRelativeLocation (Variables|Default|GetScene1) (Variables|Default|GetCameraPosition) false false))

(event Custom|座席B
  (Variables|Default|SetCameraPosition "-2167.000000,-80.000000,247.000000")
  (Rendering|SetVisibility (Variables|Default|GetPassenger_B) false false)
  (Rendering|SetVisibility (Variables|Default|GetPassenger_A) true false)
  (Transformation|SetRelativeLocation (Variables|Default|GetScene1) (Variables|Default|GetCameraPosition) false false))

(event Custom|Highway_Loop
  ;[1 1 1] ループ
  (bind _isa (Utilities|FlowControl|FlipFlop)
    (:A
      _)
    (:B
      _))
  (Variables|Default|SetStationLoop _isa))

(event Custom|座席D
  (Variables|Default|SetCameraPosition "-2167.000000,80.000000,247.000000")
  (Rendering|SetVisibility (Variables|Default|GetPassenger_D) false false)
  (Rendering|SetVisibility (Variables|Default|GetPassenger_E) true false)
  (Transformation|SetRelativeLocation (Variables|Default|GetScene1) (Variables|Default|GetCameraPosition) false false))

(event Custom|SpeedDown_75to50Km
  ;[1 1 1] 速度調節
  (bind _50_to_100 (Timeline|Speed_50%20to%2075 Reverse)
    (:Update
      (Variables|/Script/PathFollow.PFPathFollowerComponent|SetSpeedDuration (Variables|Default|GetPFPathFollower) _50_to_100))))

(event Custom|SpeedDown_100to75Km
  ;[1 1 1] 速度調節
  (bind _50_to_100 (Timeline|Speed_75%20to%20100 Reverse)
    (:Update
      (Variables|/Script/PathFollow.PFPathFollowerComponent|SetSpeedDuration (Variables|Default|GetPFPathFollower) _50_to_100))))

(event Custom|無人
  (for _array_element (Variables|Default|GetPassenger_array)
    (Development|SetHiddeninGame _array_element true false)))

(event Custom|少数
  (bind _passenger_array (Variables|Default|GetPassenger_array))
  (for _array_element _passenger_array
    (Development|SetHiddeninGame _array_element false false))
  (for _index (range 0 80)
    (Development|SetHiddeninGame (Utilities|Array|Get(acopy) _passenger_array (Math|Random|RandomIntegerinRange 0 104)) true false)))

(event Custom|普通
  (bind _passenger_array (Variables|Default|GetPassenger_array))
  (for _array_element _passenger_array
    (Development|SetHiddeninGame _array_element false false))
  (for _index (range 0 53)
    (Development|SetHiddeninGame (Utilities|Array|Get(acopy) _passenger_array (Math|Random|RandomIntegerinRange 0 104)) true false)))

(event Custom|満員
  (for _array_element (Variables|Default|GetPassenger_array)
    (Development|SetHiddeninGame _array_element false false)))

(event Custom|SpeedUp_50to100Km
  ;[1 1 1] 速度調節
  (bind _50_to_100 (Timeline|Speed_50%20to%20100 Play)
    (:Update
      (Variables|/Script/PathFollow.PFPathFollowerComponent|SetSpeedDuration (Variables|Default|GetPFPathFollower) _50_to_100))))

(event EventBeginPlay
  (CallFunction|混雑度)
  (Rendering|SetVisibility (Variables|Default|GetPassenger_B) false false)
  (Utilities|FlowControl|Delay 0.2)
  (CallFunction|初期座席))

(event Input|KeyboardEvents|End
  (params (Key :type Key%20Structure :default "None"))
  (bind _pfpathfollower (Variables|Default|GetPFPathFollower))
  ;[1 1 1] 高速道路降りる
  (:Pressed
    (bind _outactors (Actor|GetAllActorswithTag "End"))
    (for _array_element _outactors
      (Class|PFPathFollowerComponent|SetPathOwner _pfpathfollower _array_element)
      (Variables|/Script/PathFollow.PFPathFollowerComponent|SetSpeedDuration _pfpathfollower 5e+02)
      (Class|PFPathFollowerComponent|Start _pfpathfollower 0.0)
      (Utilities|FlowControl|Delay 8e+01)
      (Class|PFPathFollowerComponent|Stop _pfpathfollower))))

(fn ConstructionScript)