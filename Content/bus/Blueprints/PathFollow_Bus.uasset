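; Bus actor that drives highway start, loop and end paths through a PFPathFollower, swapping path owners per phase.
; Timelines ramp SpeedDuration for the highway entry and for 50/75/100 km/h changes, reversing to slow down.
; BulletTrainWindow events set crowding (empty, few, normal, full) by hiding passenger meshes, randomly for partial loads.
; Overlaps with tagged components stream in scenery levels, unloading the previous one after a delay.
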(event OnComponentBeginOverlap(StaticMesh)
  (params (OverlappedComponent :type Primitive%20Component%20Object%20Reference) (OtherActor :type Actor%20Object%20Reference) (OtherComp :type Primitive%20Component%20Object%20Reference) (OtherBodyIndex :type Integer) (bFromSweep :type Boolean) (SweepResult :type Hit%20Result%20Structure%20%28by%20ref%29))
  (if (Components|ComponentHasTag OtherComp "Mountain")
    (Game|LoadStreamLevel(byName) "BusLevel_Mountain" true)
    (Utilities|FlowControl|Delay 2e+01)
    (Game|UnloadStreamLevel(byName) "BusLevel_City02" false)
    (elif (Components|ComponentHasTag OtherComp "City01")
      (Game|LoadStreamLevel(byName) "BusLevel_City01" true)
      (Utilities|FlowControl|Delay 2e+01)
      (Game|UnloadStreamLevel(byName) "BusLevel_Mountain" false)
      (elif (Components|ComponentHasTag OtherComp "Suburb")
        (Game|LoadStreamLevel(byName) "BusLevel_Suburb" true)
        (Utilities|FlowControl|Delay 2e+01)
        (Game|UnloadStreamLevel(byName) "BusLevel_City01" false)
        (elif (Components|ComponentHasTag OtherComp "Suburb")
          (Game|LoadStreamLevel(byName) "BusLevel_City02" true)
          (Utilities|FlowControl|Delay 2e+01)
          (Game|UnloadStreamLevel(byName) "BusLevel_Suburb" false))))))

(event Custom|Highway_End
  (bind _pfpathfollower (Variables|Default|GetPFPathFollower))
  ;[1 1 1] 高速道路降りる
  (bind _outactors (Actor|GetAllActorswithTag "End"))
  (for _array_element _outactors
    (Class|PFPathFollowerComponent|SetPathOwner _pfpathfollower _array_element)
    (Variables|/Script/PathFollow.PFPathFollowerComponent|SetSpeedDuration _pfpathfollower 5e+02)
    (Class|PFPathFollowerComponent|Start _pfpathfollower 0.0)
    (Utilities|FlowControl|Delay 8e+01)
    (Class|PFPathFollowerComponent|Stop _pfpathfollower)))

(event Custom|Highway_Start
  (bind _pfpathfollower (Variables|Default|GetPFPathFollower))
  ;[1 1 1] 高速道路乗る
  (bind _outactors (Actor|GetAllActorswithTag "Start"))
  (for _array_element _outactors
    (Class|PFPathFollowerComponent|SetPathOwner _pfpathfollower _array_element)
    (Class|PFPathFollowerComponent|Start _pfpathfollower 0.0)
    (bind _speed (Timeline|Speed_Up Play)
      (:Update
        (Variables|/Script/PathFollow.PFPathFollowerComponent|SetSpeedDuration _pfpathfollower _speed))
      (:Finished
        (CallFunction|HighwayLoop)
        (bind _foundwidgets (Widget|GetAllWidgetsOfClass "/Game/bus/VR_Spectator_Window/BusWindow.BusWindow_C" false))
        (Default|HighwaySpeedEnable _foundwidgets)))))

(event Custom|SpeedUp_75to100Km
  ;[1 1 1] 速度調節
  (bind _50_to_100 (Timeline|Speed_75%20to%20100 Play)
    (:Update
      (Variables|/Script/PathFollow.PFPathFollowerComponent|SetSpeedDuration (Variables|Default|GetPFPathFollower) _50_to_100))))

(event Custom|SpeedUP_50to75Km
  ;[1 1 1] 速度調節
  (bind _50_to_100 (Timeline|Speed_50%20to%2075 Play)
    (:Update
      (Variables|/Script/PathFollow.PFPathFollowerComponent|SetSpeedDuration (Variables|Default|GetPFPathFollower) _50_to_100))))

(event Custom|SpeedDown_100to50Km
  ;[1 1 1] 速度調節
  (bind _50_to_100 (Timeline|Speed_50%20to%20100 Reverse)
    (:Update
      (Variables|/Script/PathFollow.PFPathFollowerComponent|SetSpeedDuration (Variables|Default|GetPFPathFollower) _50_to_100))))

(event Custom|混雑度
  (|CollapseGraph_0)
  (bind _foundwidgets (Widget|GetAllWidgetsOfClass "/Game/shinkansen/VR_Spectator_Window/BulletTrainWindow.BulletTrainWindow_C" false))
  (EventDispatchers|BindEventto無人 _foundwidgets (delegate Custom|無人))
  (EventDispatchers|BindEventto少数 _foundwidgets (delegate Custom|少数))
  (EventDispatchers|BindEventto普通 _foundwidgets (delegate Custom|普通))
  (EventDispatchers|BindEventto満員 _foundwidgets (delegate Custom|満員)))

(event Custom|Highway_Loop
  (bind _pfpathfollower (Variables|Default|GetPFPathFollower))
  ;[1 1 1] ループ
  (bind _returnvalue (Actor|GetActorOfClass "/Game/bus/Blueprints/PathFollow.PathFollow_C"))
  (Class|PFPathFollowerComponent|SetPathOwner _pfpathfollower _returnvalue)
  (Variables|/Script/PathFollow.PFPathFollowerComponent|SetSpeedDuration _pfpathfollower 1.5e+03)
  (Class|PFPathFollowerComponent|Start _pfpathfollower 0.0))

(event Custom|SpeedDown_75to50Km
  ;[1 1 1] 速度調節
  (bind _50_to_100 (Timeline|Speed_50%20to%2075 Reverse)
    (:Update
      (Variables|/Script/PathFollow.PFPathFollowerComponent|SetSpeedDuration (Variables|Default|GetPFPathFollower) _50_to_100))))

(event Custom|SpeedDown_100to75Km
  ;[1 1 1] 速度調節
  (bind _50_to_100 (Timeline|Speed_75%20to%20100 Reverse)
    (:Update
      (Variables|/Script/PathFollow.PFPathFollowerComponent|SetSpeedDuration (Variables|Default|GetPFPathFollower) _50_to_100))))

(event Custom|無人
  (for _array_element (Variables|Default|GetPassengerArray)
    (Development|SetHiddeninGame _array_element true false)))

(event Custom|少数
  (bind _passengerarray (Variables|Default|GetPassengerArray))
  (for _array_element _passengerarray
    (Development|SetHiddeninGame _array_element false false))
  (for _index (range 0 80)
    (Development|SetHiddeninGame (Utilities|Array|Get(acopy) _passengerarray (Math|Random|RandomIntegerinRange 0 104)) true false)))

(event Custom|普通
  (bind _passengerarray (Variables|Default|GetPassengerArray))
  (for _array_element _passengerarray
    (Development|SetHiddeninGame _array_element false false))
  (for _index (range 0 53)
    (Development|SetHiddeninGame (Utilities|Array|Get(acopy) _passengerarray (Math|Random|RandomIntegerinRange 0 104)) true false)))

(event Custom|満員
  (for _array_element (Variables|Default|GetPassengerArray)
    (Development|SetHiddeninGame _array_element false false)))

(event Custom|SpeedUp_50to100Km
  ;[1 1 1] 速度調節
  (bind _50_to_100 (Timeline|Speed_50%20to%20100 Play)
    (:Update
      (Variables|/Script/PathFollow.PFPathFollowerComponent|SetSpeedDuration (Variables|Default|GetPFPathFollower) _50_to_100))))

(event EventBeginPlay
  ;[1 1 1] 高速道路乗る
)

(event Input|KeyboardEvents|End
  (params (Key :type Key%20Structure :default "None"))
  (bind _pfpathfollower (Variables|Default|GetPFPathFollower))
  ;[1 1 1] 高速道路降りる
  (:Pressed
    (bind _outactors (Actor|GetAllActorswithTag "End"))
    (for _array_element _outactors
      (Class|PFPathFollowerComponent|SetPathOwner _pfpathfollower _array_element)
      (Variables|/Script/PathFollow.PFPathFollowerComponent|SetSpeedDuration _pfpathfollower 5e+02)
      (Class|PFPathFollowerComponent|Start _pfpathfollower 0.0)
      (Utilities|FlowControl|Delay 8e+01)
      (Class|PFPathFollowerComponent|Stop _pfpathfollower))))

(fn ConstructionScript)