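; SubwayLevel_BP runs the VR subway ride from Ikebukuro to Tokyo, one timeline per leg.
; Each timeline moves departure and arrival station actors along Y to fake travel, updates SubwayWindow progress, and triggers sounds and announcements.
; Finished legs, except the last, stream in the next level and unload the previous.
; An emergency-stop FlipFlop halts or resumes the leg matching the widget's StationNum; other events animate player boarding and alighting.
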(event Custom|池袋to新大塚
  ;[1 1 1] 池袋から新大塚まで
  (bind (_direction _電車_駅_の動き _インジケーター) (Timeline|タイムライン_電車の動き Play)
    (:Update
      (|駅の動き_池袋 _電車_駅_の動き _インジケーター _電車_駅_の動き))
    (:Finished
      (|レベル移行_池袋))
    (:駅出現
      (|駅出現_池袋))
    (:急停車ボタン
      (|急停車ボタン_池袋))
    (:駅到着アナウンス
      (bind _returnvalue (Actor|GetActorOfClass "/Game/Subway/Kousuke_Contents/Kousuke_Subway/Subway_announce_BP.Subway_announce_BP_C"))
      (Default|到着新大塚 _returnvalue))))

(event Custom|カスタムイベント_急停車
  (Utilities|FlowControl|FlipFlop
    (:A
      (Development|PrintString "急停車")
      (Class|AtomComponent|Play (Variables|Default|GetAtom＿急停車) 0.0)
      (bind _returnvalue (Actor|GetActorOfClass "/Game/Subway/Blueprint/急停車_BP.急停車_BP_C"))
      (Rendering|SetActorHiddenInGame _returnvalue false)
      (bind _新規track_0 (Timeline|急停車 PlayFromStart)
        (:Update
          (Transformation|SetActorRelativeLocation _returnvalue _新規track_0))
        (:駅BP停止
          (bind _foundwidgets (Widget|GetAllWidgetsOfClass "/Game/Subway/VR_Spectator_Window/SubwayWindow.SubwayWindow_C" false))
          (for _array_element _foundwidgets
            (switch int (Variables|/Game/Subway/VR_Spectator_Window/SubwayWindow.SubwayWindow_C|GetStationNum _array_element)
              (:0
                ;[1 1 1] 池袋から新大塚まで
                (bind (_direction _電車_駅_の動き _インジケーター) (Timeline|タイムライン_電車の動き Stop)
                  (:Update
                    (|駅の動き_池袋 _電車_駅_の動き _インジケーター _電車_駅_の動き))
                  (:Finished
                    (|レベル移行_池袋))
                  (:駅出現
                    (|駅出現_池袋))
                  (:急停車ボタン
                    (|急停車ボタン_池袋))
                  (:駅到着アナウンス
                    (bind _returnvalue_2 (Actor|GetActorOfClass "/Game/Subway/Kousuke_Contents/Kousuke_Subway/Subway_announce_BP.Subway_announce_BP_C"))
                    (Default|到着新大塚 _returnvalue_2))))
              (:1
                ;[1 1 1] 新大塚から茗荷谷まで
                (bind (_direction_2 _電車_駅_の動き_2 _インジケーター_2) (Timeline|タイムライン_1 Stop)
                  (:Update
                    (|駅の動き_新大塚 _電車_駅_の動き_2 _インジケーター_2 _電車_駅_の動き_2))
                  (:Finished
                    (|レベル移行_新大塚))
                  (:駅出現
                    (|駅出現_新大塚))
                  (:急停車ボタン
                    (|急停車ボタン_新大塚))
                  (:駅到着アナウンス
                    (bind _returnvalue_3 (Actor|GetActorOfClass "/Game/Subway/Kousuke_Contents/Kousuke_Subway/Subway_announce_BP.Subway_announce_BP_C"))
                    (Default|到着茗荷谷 _returnvalue_3))))
              (:2
                ;[1 1 1] 茗荷谷から後楽園まで
                (bind (_direction_3 _電車_駅_の動き_3 _インジケーター_3) (Timeline|タイムライン_2 Stop)
                  (:Update
                    (|駅の動き_茗荷谷 _電車_駅_の動き_3 _インジケーター_3 _電車_駅_の動き_3))
                  (:Finished
                    (|レベル移行_茗荷谷))
                  (:駅出現
                    (|駅出現_茗荷谷))
                  (:急停車ボタン
                    (|急停車ボタン_茗荷谷))
                  (:駅到着アナウンス
                    (bind _returnvalue_4 (Actor|GetActorOfClass "/Game/Subway/Kousuke_Contents/Kousuke_Subway/Subway_announce_BP.Subway_announce_BP_C"))
                    (Default|到着後楽園 _returnvalue_4))))
              (:3
                ;[1 1 1] 後楽園から本郷まで
                (bind (_direction_4 _電車_駅_の動き_4 _インジケーター_4) (Timeline|タイムライン_3 Stop)
                  (:Update
                    (|駅の動き_後楽園 _電車_駅_の動き_4 _インジケーター_4 _電車_駅_の動き_4))
                  (:Finished
                    (|レベル移行_後楽園))
                  (:駅出現
                    (|駅出現_後楽園))
                  (:急停車ボタン
                    (|急停車ボタン_後楽園))
                  (:駅到着アナウンス
                    (bind _returnvalue_5 (Actor|GetActorOfClass "/Game/Subway/Kousuke_Contents/Kousuke_Subway/Subway_announce_BP.Subway_announce_BP_C"))
                    (Default|到着本郷三丁目 _returnvalue_5))))
              (:4
                ;[1 1 1] 本郷から御茶ノ水
                (bind (_direction_5 _電車_駅_の動き_5 _インジケーター_5) (Timeline|タイムライン_4 Stop)
                  (:Update
                    (|駅の動き_本郷三丁目 _電車_駅_の動き_5 _インジケーター_5 _電車_駅_の動き_5))
                  (:Finished
                    (|レベル移行_本郷三丁目))
                  (:駅出現
                    (|駅出現_本郷三丁目))
                  (:急停車ボタン
                    (|急停車ボタン_本郷三丁目))
                  (:駅到着アナウンス
                    (bind _returnvalue_6 (Actor|GetActorOfClass "/Game/Subway/Kousuke_Contents/Kousuke_Subway/Subway_announce_BP.Subway_announce_BP_C"))
                    (Default|到着御茶ノ水 _returnvalue_6))))
              (:5
                ;[1 1 1] 御茶ノ水から淡路町まで
                (bind (_direction_6 _電車_駅_の動き_6 _インジケーター_6) (Timeline|タイムライン_5 Stop)
                  (:Update
                    (|駅の動き_御茶ノ水 _電車_駅_の動き_6 _電車_駅_の動き_6 _インジケーター_6))
                  (:Finished
                    (|レベル移行_御茶ノ水))
                  (:駅出現
                    (|駅出現_御茶ノ水))
                  (:急停車ボタン
                    (|急停車ボタン_御茶ノ水))
                  (:駅到着アナウンス
                    (bind _returnvalue_7 (Actor|GetActorOfClass "/Game/Subway/Kousuke_Contents/Kousuke_Subway/Subway_announce_BP.Subway_announce_BP_C"))
                    (Default|到着淡路町 _returnvalue_7))))
              (:6
                ;[1 1 1] 淡路町から大手町
                (bind (_direction_7 _電車_駅_の動き_7 _インジケーター_7) (Timeline|タイムライン_6 Stop)
                  (:Update
                    (|駅の動き_淡路町 _電車_駅_の動き_7 _インジケーター_7 _電車_駅_の動き_7))
                  (:Finished
                    (|レベル移行_淡路町))
                  (:駅出現
                    (|駅出現_淡路町))
                  (:急停車ボタン
                    (|急停車ボタン_淡路町))
                  (:駅到着アナウンス
                    (bind _returnvalue_8 (Actor|GetActorOfClass "/Game/Subway/Kousuke_Contents/Kousuke_Subway/Subway_announce_BP.Subway_announce_BP_C"))
                    (Default|到着大手町 _returnvalue_8))))
              (:7
                ;[1 1 1] 淡路町から大手町
                (bind (_direction_8 _電車_駅_の動き_8 _新規track_0_2) (Timeline|タイムライン_7 Stop)
                  (:Update
                    (|駅の動き_大手町 _電車_駅_の動き_8 _新規track_0_2 _電車_駅_の動き_8))
                  (:駅出現
                    (|駅出現_大手町))
                  (:急停車ボタン
                    (|急停車ボタン_大手町))
                  (:駅到着アナウンス
                    (bind _returnvalue_9 (Actor|GetActorOfClass "/Game/Subway/Kousuke_Contents/Kousuke_Subway/Subway_announce_BP.Subway_announce_BP_C"))
                    (Default|到着東京 _returnvalue_9)))))))))
    (:B
      (Utilities|FlowControl|Sequence
        (:then_0
          (bind _foundwidgets_2 (Widget|GetAllWidgetsOfClass "/Game/Subway/VR_Spectator_Window/SubwayWindow.SubwayWindow_C" false))
          (for _array_element_2 _foundwidgets_2
            (switch int (Variables|/Game/Subway/VR_Spectator_Window/SubwayWindow.SubwayWindow_C|GetStationNum _array_element_2)
              (:0
                (Timeline|タイムライン_電車の動き Play))
              (:1
                (Timeline|タイムライン_1 Play))
              (:2
                (Timeline|タイムライン_2 Play))
              (:3
                (Timeline|タイムライン_3 Play))
              (:4
                (Timeline|タイムライン_4 Play))
              (:5
                (Timeline|タイムライン_5 Play))
              (:6
                (Timeline|タイムライン_6 Play))
              (:7
                (Timeline|タイムライン_7 Play)))))
        (:then_1
          (bind _トンネル移動 (Timeline|タイムライン_9 PlayFromStart)
            (:Update
              (Transformation|SetActorRelativeLocation _returnvalue _トンネル移動))
            (:Finished
              (Rendering|SetActorHiddenInGame _returnvalue true))))))))

(event Custom|大手町to東京
  ;[1 1 1] 淡路町から大手町
  (bind (_direction _電車_駅_の動き _新規track_0) (Timeline|タイムライン_7 Play)
    (:Update
      (|駅の動き_大手町 _電車_駅_の動き _新規track_0 _電車_駅_の動き))
    (:駅出現
      (|駅出現_大手町))
    (:急停車ボタン
      (|急停車ボタン_大手町))
    (:駅到着アナウンス
      (bind _returnvalue (Actor|GetActorOfClass "/Game/Subway/Kousuke_Contents/Kousuke_Subway/Subway_announce_BP.Subway_announce_BP_C"))
      (Default|到着東京 _returnvalue))))

(event Custom|乗車_左
  ;[1 1 1] プレイヤー下車
  (|左側乗車下車アニメーション) ; enters at ReverseFromEnd
)

(event Custom|下車_L
  (bind _returnvalue (Actor|GetActorOfClass "/Game/NaReRu_Common/VR_Character/VRPlayer_Character.VRPlayer_Character_C"))
  ;[1 1 1] 淡路町から大手町
  (Variables|/Game/NaReRu_Common/VR_Character/VRPlayer_Character.VRPlayer_Character_C|SetVRCameraHight _returnvalue (+ (Variables|/Game/NaReRu_Common/VR_Character/VRPlayer_Character.VRPlayer_Character_C|GetVRCameraHight _returnvalue) 4e+01))
  (Default|身長変更 _returnvalue)
  (bind (_direction _移動 _ローテーション) (Timeline|タイムライン_0 ReverseFromEnd)
    (:Update
      (bind _returnvalue_2 (Actor|GetActorOfClass "/Game/NaReRu_Common/VR_Character/VRPlayer_Character.VRPlayer_Character_C"))
      (Transformation|SetActorLocationAndRotation _returnvalue_2 (Math|Vector|MakeVector (.X (Math|Vector|BreakVector _移動)) (.Y (Math|Vector|BreakVector _移動)) (.Z (Math|Vector|BreakVector (Transformation|GetActorLocation (Game|GetPlayerCharacter 0))))) (Math|Rotator|MakeRotator 0.0 0.0 (.z _ローテーション)) true))))

(event Custom|下車_左
  ;[1 1 1] プレイヤー下車
  (Development|PrintString "下車")
  (|左側乗車下車アニメーション))

(event Custom|茗荷谷to後楽園
  ;[1 1 1] 茗荷谷から後楽園まで
  (bind (_direction _電車_駅_の動き _インジケーター) (Timeline|タイムライン_2 Play)
    (:Update
      (|駅の動き_茗荷谷 _電車_駅_の動き _インジケーター _電車_駅_の動き))
    (:Finished
      (|レベル移行_茗荷谷))
    (:駅出現
      (|駅出現_茗荷谷))
    (:急停車ボタン
      (|急停車ボタン_茗荷谷))
    (:駅到着アナウンス
      (bind _returnvalue (Actor|GetActorOfClass "/Game/Subway/Kousuke_Contents/Kousuke_Subway/Subway_announce_BP.Subway_announce_BP_C"))
      (Default|到着後楽園 _returnvalue))))

(event Custom|後楽園to本郷
  ;[1 1 1] 後楽園から本郷まで
  (bind (_direction _電車_駅_の動き _インジケーター) (Timeline|タイムライン_3 Play)
    (:Update
      (|駅の動き_後楽園 _電車_駅_の動き _インジケーター _電車_駅_の動き))
    (:Finished
      (|レベル移行_後楽園))
    (:駅出現
      (|駅出現_後楽園))
    (:急停車ボタン
      (|急停車ボタン_後楽園))
    (:駅到着アナウンス
      (bind _returnvalue (Actor|GetActorOfClass "/Game/Subway/Kousuke_Contents/Kousuke_Subway/Subway_announce_BP.Subway_announce_BP_C"))
      (Default|到着本郷三丁目 _returnvalue))))

(event Custom|本郷to御茶ノ水
  ;[1 1 1] 本郷から御茶ノ水
  (bind (_direction _電車_駅_の動き _インジケーター) (Timeline|タイムライン_4 Play)
    (:Update
      (|駅の動き_本郷三丁目 _電車_駅_の動き _インジケーター _電車_駅_の動き))
    (:Finished
      (|レベル移行_本郷三丁目))
    (:駅出現
      (|駅出現_本郷三丁目))
    (:急停車ボタン
      (|急停車ボタン_本郷三丁目))
    (:駅到着アナウンス
      (bind _returnvalue (Actor|GetActorOfClass "/Game/Subway/Kousuke_Contents/Kousuke_Subway/Subway_announce_BP.Subway_announce_BP_C"))
      (Default|到着御茶ノ水 _returnvalue))))

(event Custom|御茶ノ水to淡路町
  ;[1 1 1] 御茶ノ水から淡路町まで
  (bind (_direction _電車_駅_の動き _インジケーター) (Timeline|タイムライン_5 Play)
    (:Update
      (|駅の動き_御茶ノ水 _電車_駅_の動き _電車_駅_の動き _インジケーター))
    (:Finished
      (|レベル移行_御茶ノ水))
    (:駅出現
      (|駅出現_御茶ノ水))
    (:急停車ボタン
      (|急停車ボタン_御茶ノ水))
    (:駅到着アナウンス
      (bind _returnvalue (Actor|GetActorOfClass "/Game/Subway/Kousuke_Contents/Kousuke_Subway/Subway_announce_BP.Subway_announce_BP_C"))
      (Default|到着淡路町 _returnvalue))))

(event Custom|乗車
  ;[1 1 1] プレイヤー下車
  (Default|Call乗車R)
  (bind _outactors (Actor|GetAllActorsOfClass "SubwayLevel_BP_C"))
  (EventDispatchers|BindEventto乗車L _outactors (delegate Custom|乗車_左)))

(event Custom|淡路町to大手町
  ;[1 1 1] 淡路町から大手町
  (bind (_direction _電車_駅_の動き _インジケーター) (Timeline|タイムライン_6 Play)
    (:Update
      (|駅の動き_淡路町 _電車_駅_の動き _インジケーター _電車_駅_の動き))
    (:Finished
      (|レベル移行_淡路町))
    (:駅出現
      (|駅出現_淡路町))
    (:急停車ボタン
      (|急停車ボタン_淡路町))
    (:駅到着アナウンス
      (bind _returnvalue (Actor|GetActorOfClass "/Game/Subway/Kousuke_Contents/Kousuke_Subway/Subway_announce_BP.Subway_announce_BP_C"))
      (Default|到着大手町 _returnvalue))))

(event Custom|新大塚to茗荷谷
  ;[1 1 1] 新大塚から茗荷谷まで
  (bind (_direction _電車_駅_の動き _インジケーター) (Timeline|タイムライン_1 Play)
    (:Update
      (|駅の動き_新大塚 _電車_駅_の動き _インジケーター _電車_駅_の動き))
    (:Finished
      (|レベル移行_新大塚))
    (:駅出現
      (|駅出現_新大塚))
    (:急停車ボタン
      (|急停車ボタン_新大塚))
    (:駅到着アナウンス
      (bind _returnvalue (Actor|GetActorOfClass "/Game/Subway/Kousuke_Contents/Kousuke_Subway/Subway_announce_BP.Subway_announce_BP_C"))
      (Default|到着茗荷谷 _returnvalue))))

(event EventBeginPlay
  (bind _returnvalue (Actor|GetActorOfClass "/Game/Subway/Blueprint/急停車_BP.急停車_BP_C"))
  (Rendering|SetActorHiddenInGame _returnvalue true))

(fn ConstructionScript)